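; BP_CameraTrigger is a placeable trigger volume that switches the camera target for actors entering it.
; Box overlap sends SetNewCamTargetMessage to the overlapping actor, passing the trigger's own Camera on enter and an empty target on exit, both with zero offset.
; The construction script sizes the box from CollisionSize and positions the camera from CamTransform, which BeginPlay reapplies.
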(event OnComponentBeginOverlap(Box)
  (params (OverlappedComponent :type Primitive%20Component%20Object%20Reference) (OtherActor :type Actor%20Object%20Reference) (OtherComp :type Primitive%20Component%20Object%20Reference) (OtherBodyIndex :type Integer) (bFromSweep :type Boolean) (SweepResult :type Hit%20Result%20Structure%20%28by%20ref%29))
  (Class|BPIDarkPictures|SetNewCamTarget(Message) OtherActor (Variables|Default|GetCamera) "0, 0, 0"))

(event OnComponentEndOverlap(Box)
  (params (OverlappedComponent :type Primitive%20Component%20Object%20Reference) (OtherActor :type Actor%20Object%20Reference) (OtherComp :type Primitive%20Component%20Object%20Reference) (OtherBodyIndex :type Integer))
  (Class|BPIDarkPictures|SetNewCamTarget(Message) OtherActor 0 "0, 0, 0"))

(event EventBeginPlay
  (Transformation|SetRelativeTransform (Variables|Default|GetCamera) (Variables|Default|Get_camTransform) false true))

(fn ConstructionScript
  (Transformation|SetRelativeTransform (Variables|Default|GetCamera) (Variables|Default|Get_camTransform) false true)
  (Components|Box|SetBoxExtent (Variables|Default|GetBox) (Variables|Default|Get_CollisionSize) true))