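; BP_MasterCharacter is a character Blueprint whose camera and movement are configured from a Data Asset.
; On BeginPlay it copies the asset's settings to the spring arm length, camera projection, FOV, near clip and walk speed.
; Orthographic width is derived by scaling the same FOV value.
; The CanJump flag only sets MaxJumpApexAttemptsPerSimulation, a simulation setting, rather than the jump count.
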(event EventBeginPlay
  (bind __dataasset (Variables|Default|Get_dataAsset))
  (bind _camera (Variables|Default|GetCamera))
  (bind __dataasset_2 (Variables|Default|Get_dataAsset))
  (bind _charactermovement (Variables|Character|GetCharacterMovement))
  (bind _fov (Variables|/Game/_Manager/DataAsset/BP/BP_DataAsset.BP_DataAsset_C|GetFOV __dataasset))
  ;[1 0 0] Data Asset
  (Variables|/Script/Engine.SpringArmComponent|SetTargetArmLength (Variables|Default|GetSpringArm) (Variables|/Game/_Manager/DataAsset/BP/BP_DataAsset.BP_DataAsset_C|Getdistance __dataasset_2))
  (Class|CameraComponent|SetProjectionMode _camera (select (Variables|/Game/_Manager/DataAsset/BP/BP_DataAsset.BP_DataAsset_C|Getorthographic __dataasset_2) "Orthographic" "Perspective"))
  (Camera|SetFieldOfView _camera _fov)
  (Class|CameraComponent|SetOrthoWidth _camera (* _fov 5.6))
  (Class|CameraComponent|SetOrthoNearClipPlane _camera (Variables|/Game/_Manager/DataAsset/BP/BP_DataAsset.BP_DataAsset_C|Getclipping __dataasset))
  (Variables|/Script/Engine.CharacterMovementComponent|SetMaxWalkSpeed _charactermovement (Variables|/Game/_Manager/DataAsset/BP/BP_DataAsset.BP_DataAsset_C|GetwalkSpeed __dataasset))
  (Variables|/Script/Engine.CharacterMovementComponent|SetMaxJumpApexAttemptsPerSimulation _charactermovement (Math|Integer|SelectInt 1 0 (Variables|/Game/_Manager/DataAsset/BP/BP_DataAsset.BP_DataAsset_C|GetcanJump __dataasset))))

(fn ConstructionScript)